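; BP_Obstacles_Car4 is a runner obstacle that kills the player character on overlap unless it is sliding.
; On actor overlap it casts to BP_RunnerCharacter and checks IsSliding.
; If the character is not sliding, it calls Death on it, then pauses the game after a short delay.
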(event `self.ReceiveActorBeginOverlap`
  (params (OtherActor :type "Actor Object Reference"))
  (bind _asbp_runner_character (cast `/Game/Runner/Blueprints/BP_RunnerCharacter` OtherActor))
  (if (not (`/Game/Runner/Blueprints/BP_RunnerCharacter.Is Sliding` _asbp_runner_character))
    (`/Game/Runner/Blueprints/BP_RunnerCharacter.Death` _asbp_runner_character)
    (`KismetSystemLibrary.Delay` 1.0)
    (`GameplayStatics.SetGamePaused` true)))

(fn `UserConstructionScript`
  (`parent.UserConstructionScript`))