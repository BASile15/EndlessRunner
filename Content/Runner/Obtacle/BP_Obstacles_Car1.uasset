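; BP_Obstacles_Car1 is a runner-game car obstacle that moves when the player approaches and kills them on contact.
; On BeginPlay it destroys actors overlapping BoxOverlap that fail an equality check against BP_Coin.
; When the runner enters that box, a Timeline lerps the mesh's X toward an Arrow marker, then the obstacle destroys itself after a delay.
; CarCollision overlap calls the runner's Death, then pauses the game after a delay.
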(event `self.ReceiveBeginPlay`
  (for _array_element (`PrimitiveComponent.GetOverlappingActors` (`self.Box overlap`) "/Script/Engine.Actor")
    (if (not (== _array_element "/Game/Runner/Blueprints/BP_Coin.BP_Coin"))
      (`self.K2_DestroyActor` _array_element))))

(event `self.Car Collision.OnComponentBeginOverlap`
  (params (OverlappedComponent :type "PrimitiveComponent Object Reference") (OtherActor :type "Actor Object Reference") (OtherComp :type "PrimitiveComponent Object Reference") (OtherBodyIndex :type Integer) (bFromSweep :type Boolean) (SweepResult :type "HitResult Structure (by ref)"))
  (bind _asbp_runner_character (cast `/Game/Runner/Blueprints/BP_RunnerCharacter` OtherActor))
  (`/Game/Runner/Blueprints/BP_RunnerCharacter.Death` _asbp_runner_character)
  (`KismetSystemLibrary.Delay` 1.0)
  (`GameplayStatics.SetGamePaused` true))

(event `self.Box overlap.OnComponentBeginOverlap`
  (params (OverlappedComponent :type "PrimitiveComponent Object Reference") (OtherActor :type "Actor Object Reference") (OtherComp :type "PrimitiveComponent Object Reference") (OtherBodyIndex :type Integer) (bFromSweep :type Boolean) (SweepResult :type "HitResult Structure (by ref)"))
  (bind _staticmesh (`self.StaticMesh`))
  (cast `/Game/Runner/Blueprints/BP_RunnerCharacter` OtherActor)
  (bind (_direction _mouve_obstacle) (`Timeline|Timeline` :!via `PlayFromStart`)
    (:`Update`
      (`SceneComponent.K2_SetWorldLocation` _staticmesh (`KismetMathLibrary.MakeVector` (`KismetMathLibrary.Lerp` (.x (`SceneComponent.K2_GetComponentLocation` _staticmesh)) (.x (`SceneComponent.K2_GetComponentLocation` (`self.Arrow`))) _mouve_obstacle) (.y (`SceneComponent.K2_GetComponentLocation` _staticmesh)) (.z (`SceneComponent.K2_GetComponentLocation` _staticmesh))) false false))
    (:`Finished`
      (`KismetSystemLibrary.Delay` 5.0)
      (`self.K2_DestroyActor`))))

(fn `UserConstructionScript`
  (`parent.UserConstructionScript`))