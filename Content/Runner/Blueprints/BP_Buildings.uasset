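; Modular building segment for an endless runner that fills itself with randomized scenery.
; The construction script calls SpawnBuildings, which adds a randomly chosen child actor, one of seven options, at each of six spawn points (SP1 to SP6).
; Overlapping the Box trigger asks BP_RunnerGameMode to extend the buildings.
; GetAttachPoint exposes the Arrow's world transform, presumably as the connection point for the next segment.
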(event `self.Box.OnComponentBeginOverlap`
  (params (OverlappedComponent :type "PrimitiveComponent Object Reference") (OtherActor :type "Actor Object Reference") (OtherComp :type "PrimitiveComponent Object Reference") (OtherBodyIndex :type Integer) (bFromSweep :type Boolean) (SweepResult :type "HitResult Structure (by ref)"))
  ; Extend Buildings
  (bind _asbp_runner_game_mode (cast `/Game/Runner/Blueprints/BP_RunnerGameMode` (`GameplayStatics.GetGameMode`)))
  (`/Game/Runner/Blueprints/BP_RunnerGameMode.Extend Buildings` _asbp_runner_game_mode))

(fn `Get AttachPoint`
  (returns (ReturnValue :type "Transform Structure"))
  (return (`SceneComponent.K2_GetComponentToWorld` (`self.Arrow`))))

(fn `SpawnBuildings`
  (bind _returnvalue (`SceneComponent.GetRelativeTransform` (`self.SP2`)))
  (bind _returnvalue_2 (`SceneComponent.GetRelativeTransform` (`self.SP3`)))
  (bind _returnvalue_3 (`SceneComponent.GetRelativeTransform` (`self.SP6`)))
  (bind _returnvalue_4 (`SceneComponent.GetRelativeTransform` (`self.SP4`)))
  (bind _returnvalue_5 (`SceneComponent.GetRelativeTransform` (`self.SP5`)))
  (bind _returnvalue_6 (`SceneComponent.GetRelativeTransform` (`self.SP1`)))
  (`|ExecutionSequence`
    (:`then_0`
      (switch `int` (`KismetMathLibrary.RandomIntegerInRange` 0 6)
        (:`0`
          (`AddComponent|NODE_AddChildActorComponent-13` :`RelativeTransform` _returnvalue_6))
        (:`1`
          (`AddComponent|NODE_AddChildActorComponent-16` :`RelativeTransform` _returnvalue_6))
        (:`2`
          (`AddComponent|NODE_AddChildActorComponent-17` :`RelativeTransform` _returnvalue_6))
        (:`3`
          (`AddComponent|NODE_AddChildActorComponent-18` :`RelativeTransform` _returnvalue_6))
        (:`4`
          (`AddComponent|NODE_AddChildActorComponent-19` :`RelativeTransform` _returnvalue_6))
        (:`5`
          (`AddComponent|NODE_AddChildActorComponent-20` :`RelativeTransform` _returnvalue_6))
        (:`6`
          (`AddComponent|NODE_AddChildActorComponent-21` :`RelativeTransform` _returnvalue_6))))
    (:`then_1`
      (switch `int` (`KismetMathLibrary.RandomIntegerInRange` 0 6)
        (:`0`
          (`AddComponent|NODE_AddChildActorComponent-22` :`RelativeTransform` _returnvalue))
        (:`1`
          (`AddComponent|NODE_AddChildActorComponent-23` :`RelativeTransform` _returnvalue))
        (:`2`
          (`AddComponent|NODE_AddChildActorComponent-24` :`RelativeTransform` _returnvalue))
        (:`3`
          (`AddComponent|NODE_AddChildActorComponent-25` :`RelativeTransform` _returnvalue))
        (:`4`
          (`AddComponent|NODE_AddChildActorComponent-26` :`RelativeTransform` _returnvalue))
        (:`5`
          (`AddComponent|NODE_AddChildActorComponent-27` :`RelativeTransform` _returnvalue))
        (:`6`
          (`AddComponent|NODE_AddChildActorComponent-28` :`RelativeTransform` _returnvalue))))
    (:`then_2`
      (switch `int` (`KismetMathLibrary.RandomIntegerInRange` 0 6)
        (:`0`
          (`AddComponent|NODE_AddChildActorComponent-29` :`RelativeTransform` _returnvalue_2))
        (:`1`
          (`AddComponent|NODE_AddChildActorComponent-30` :`RelativeTransform` _returnvalue_2))
        (:`2`
          (`AddComponent|NODE_AddChildActorComponent-31` :`RelativeTransform` _returnvalue_2))
        (:`3`
          (`AddComponent|NODE_AddChildActorComponent-32` :`RelativeTransform` _returnvalue_2))
        (:`4`
          (`AddComponent|NODE_AddChildActorComponent-33` :`RelativeTransform` _returnvalue_2))
        (:`5`
          (`AddComponent|NODE_AddChildActorComponent-34` :`RelativeTransform` _returnvalue_2))
        (:`6`
          (`AddComponent|NODE_AddChildActorComponent-35` :`RelativeTransform` _returnvalue_2))))
    (:`then_3`
      (switch `int` (`KismetMathLibrary.RandomIntegerInRange` 0 6)
        (:`0`
          (`AddComponent|NODE_AddChildActorComponent-36` :`RelativeTransform` _returnvalue_4))
        (:`1`
          (`AddComponent|NODE_AddChildActorComponent-37` :`RelativeTransform` _returnvalue_4))
        (:`2`
          (`AddComponent|NODE_AddChildActorComponent-38` :`RelativeTransform` _returnvalue_4))
        (:`3`
          (`AddComponent|NODE_AddChildActorComponent-39` :`RelativeTransform` _returnvalue_4))
        (:`4`
          (`AddComponent|NODE_AddChildActorComponent-40` :`RelativeTransform` _returnvalue_4))
        (:`5`
          (`AddComponent|NODE_AddChildActorComponent-41` :`RelativeTransform` _returnvalue_4))
        (:`6`
          (`AddComponent|NODE_AddChildActorComponent-42` :`RelativeTransform` _returnvalue_4))))
    (:`then_4`
      (switch `int` (`KismetMathLibrary.RandomIntegerInRange` 0 6)
        (:`0`
          (`AddComponent|NODE_AddChildActorComponent-43` :`RelativeTransform` _returnvalue_5))
        (:`1`
          (`AddComponent|NODE_AddChildActorComponent-44` :`RelativeTransform` _returnvalue_5))
        (:`2`
          (`AddComponent|NODE_AddChildActorComponent-45` :`RelativeTransform` _returnvalue_5))
        (:`3`
          (`AddComponent|NODE_AddChildActorComponent-46` :`RelativeTransform` _returnvalue_5))
        (:`4`
          (`AddComponent|NODE_AddChildActorComponent-47` :`RelativeTransform` _returnvalue_5))
        (:`5`
          (`AddComponent|NODE_AddChildActorComponent-48` :`RelativeTransform` _returnvalue_5))
        (:`6`
          (`AddComponent|NODE_AddChildActorComponent-49` :`RelativeTransform` _returnvalue_5))))
    (:`then_5`
      (switch `int` (`KismetMathLibrary.RandomIntegerInRange` 0 6)
        (:`0`
          (`AddComponent|NODE_AddChildActorComponent-50` :`RelativeTransform` _returnvalue_3))
        (:`1`
          (`AddComponent|NODE_AddChildActorComponent-51` :`RelativeTransform` _returnvalue_3))
        (:`2`
          (`AddComponent|NODE_AddChildActorComponent-52` :`RelativeTransform` _returnvalue_3))
        (:`3`
          (`AddComponent|NODE_AddChildActorComponent-53` :`RelativeTransform` _returnvalue_3))
        (:`4`
          (`AddComponent|NODE_AddChildActorComponent-54` :`RelativeTransform` _returnvalue_3))
        (:`5`
          (`AddComponent|NODE_AddChildActorComponent-55` :`RelativeTransform` _returnvalue_3))
        (:`6`
          (`AddComponent|NODE_AddChildActorComponent-56` :`RelativeTransform` _returnvalue_3))))))

(fn `UserConstructionScript`
  (`self.SpawnBuildings`))