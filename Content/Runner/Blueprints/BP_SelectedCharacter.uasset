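; Character-selection display actor for the runner game that previews Manny, Kevin and Camila and records which one is chosen.
; Show events toggle component visibility so only the named character is visible.
; Spawn events spawn nothing; they store that character's asset in SelectedCharacter on BP_GameInstance, with Kevin mapped to the Runner asset.
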(event `Show Manny`
  (`SceneComponent.SetHiddenInGame` (`self.Manny`) false false)
  (`SceneComponent.SetHiddenInGame` (`self.Kevin`) true false)
  (`SceneComponent.SetHiddenInGame` (`self.Camila`) true false))

(event `Show Kevin`
  (`SceneComponent.SetHiddenInGame` (`self.Kevin`) false false)
  (`SceneComponent.SetHiddenInGame` (`self.Camila`) true false)
  (`SceneComponent.SetHiddenInGame` (`self.Manny`) true false))

(event `Show Camila`
  (`SceneComponent.SetHiddenInGame` (`self.Camila`) false false)
  (`SceneComponent.SetHiddenInGame` (`self.Manny`) true false)
  (`SceneComponent.SetHiddenInGame` (`self.Kevin`) true false))

(event `Spawn Manny`
  (bind _asbp_game_instance (cast `/Game/Runner/Blueprints/BP_GameInstance` (`GameplayStatics.GetGameInstance`)))
  (set `/Game/Runner/Blueprints/BP_GameInstance.SelectedCharacter` "/Game/Characters/Mannequins/Meshes/SKM_Manny_Simple.SKM_Manny_Simple" _asbp_game_instance))

(event `Spawn Kevin`
  (bind _asbp_game_instance (cast `/Game/Runner/Blueprints/BP_GameInstance` (`GameplayStatics.GetGameInstance`)))
  (set `/Game/Runner/Blueprints/BP_GameInstance.SelectedCharacter` "/Game/Runner/Character/Kevin/Runner.Runner" _asbp_game_instance))

(event `Spawn Camila`
  (bind _asbp_game_instance (cast `/Game/Runner/Blueprints/BP_GameInstance` (`GameplayStatics.GetGameInstance`)))
  (set `/Game/Runner/Blueprints/BP_GameInstance.SelectedCharacter` "/Game/Runner/Character/Camila/Camila.Camila" _asbp_game_instance))

(fn `UserConstructionScript`)