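; Hoverboard power-up pickup for the runner, granting the player a roughly ten-second hover.
; Player overlap plays a sound, hides the pickup and, unless already hovering, sets IsHovering, shows the character's board and resets HoverTime on BP_RunnerGameMode.
; A delayed loop counts HoverTime down; a parallel delay or lost hover state ends the effect and destroys the pickup.
; The pickup also destroys itself when overlapping wall, blocker or car obstacles.
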(event `self.Hoverboard.OnComponentBeginOverlap`
  (params (OverlappedComponent :type "PrimitiveComponent Object Reference") (OtherActor :type "Actor Object Reference") (OtherComp :type "PrimitiveComponent Object Reference") (OtherBodyIndex :type Integer) (bFromSweep :type Boolean) (SweepResult :type "HitResult Structure (by ref)"))
  (`|ExecutionSequence`
    (:`then_0`
      (bind _asbp_runner_character (cast `/Game/Runner/Blueprints/BP_RunnerCharacter` OtherActor))
      (bind _asbp_runner_game_mode (cast `/Game/Runner/Blueprints/BP_RunnerGameMode` (`GameplayStatics.GetGameMode`)))
      (`GameplayStatics.PlaySound2D` "/Game/Runner/Meshes/350874__cabled_mess__coin_c_08.350874__cabled_mess__coin_c_08" 1.0 1.0 0.0 null null)
      (`self.SetActorHiddenInGame` true)
      (if (not (`/Game/Runner/Blueprints/BP_RunnerCharacter.is Hovering` _asbp_runner_character))
        (set `/Game/Runner/Blueprints/BP_RunnerGameMode.Hover Time` 10.0 _asbp_runner_game_mode)
        (set `/Game/Runner/Blueprints/BP_RunnerCharacter.is Hovering` true _asbp_runner_character)
        (`SceneComponent.SetHiddenInGame` (`/Game/Runner/Blueprints/BP_RunnerCharacter.hoverboard` _asbp_runner_character) false false)
        (`|ExecutionSequence`
          (:`then_0`
            (`/Game/Runner/Blueprints/ForLoopDelay.ForLoopWithDelay` 0 10 1.0
              (:`Loop Body`
                (bind _asbp_runner_character_2 (cast `/Game/Runner/Blueprints/BP_RunnerCharacter` (`GameplayStatics.GetPlayerCharacter` 0)))
                (if (`/Game/Runner/Blueprints/BP_RunnerCharacter.is Hovering` _asbp_runner_character_2)
                  (bind _result (`/Engine/EditorBlueprintResources/StandardMacros.DecrementFloat` (`/Game/Runner/Blueprints/BP_RunnerGameMode.Hover Time` _asbp_runner_game_mode))
                    (:`  `
                      (set `/Game/Runner/Blueprints/BP_RunnerGameMode.Hover Time` (`KismetMathLibrary.FMax` _result) _asbp_runner_game_mode)))
                  (else
                    (bind _asbp_runner_character_3 (cast `/Game/Runner/Blueprints/BP_RunnerCharacter` (`GameplayStatics.GetPlayerCharacter` 0) :!label _label))
                    (set `/Game/Runner/Blueprints/BP_RunnerCharacter.is Hovering` false _asbp_runner_character_3)
                    (`SceneComponent.SetHiddenInGame` (`/Game/Runner/Blueprints/BP_RunnerCharacter.hoverboard` _asbp_runner_character_3) true false)
                    (`self.K2_DestroyActor`))))))
          (:`then_1`
            (`KismetSystemLibrary.Delay` 10.2)
            (goto _label)))))
    (:`then_1`
      (cast `/Game/Runner/Obtacle/BP_Obstacles_Wall` OtherActor)
      (`self.K2_DestroyActor`))
    (:`then_2`
      (cast `/Game/Runner/Obtacle/BP_Obstacles_Blocker` OtherActor)
      (`self.K2_DestroyActor`))
    (:`then_3`
      (cast `/Game/Runner/Obtacle/BP_Obstacles_Car1` OtherActor)
      (`self.K2_DestroyActor`))
    (:`then_4`
      (cast `/Game/Runner/Obtacle/BP_Obstacles_Car2` OtherActor)
      (`self.K2_DestroyActor`))
    (:`then_5`
      (cast `/Game/Runner/Obtacle/BP_Obstacles_Car3` OtherActor)
      (`self.K2_DestroyActor`))
    (:`then_6`
      (cast `/Game/Runner/Obtacle/BP_Obstacles_Car4` OtherActor)
      (`self.K2_DestroyActor`))))

(fn `UserConstructionScript`)