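; Runner obstacle destroyer that clears obstacles it overlaps while the player character is hovering or dead.
; On overlap it checks the player's state, then a Sequence of casts destroys wall, blocker or any of four car obstacle types.
; After destroying an obstacle it removes itself following a short shared delay.
; If the player is neither hovering nor dead, any overlap makes it destroy itself immediately.
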(event `self.ReceiveActorBeginOverlap`
  (params (OtherActor :type "Actor Object Reference"))
  (bind _asbp_runner_character (cast `/Game/Runner/Blueprints/BP_RunnerCharacter` (`GameplayStatics.GetPlayerCharacter` 0)))
  (if (or (`/Game/Runner/Blueprints/BP_RunnerCharacter.is Hovering` _asbp_runner_character) (`/Game/Runner/Blueprints/BP_RunnerCharacter.is dead` _asbp_runner_character))
    (`|ExecutionSequence`
      (:`then_0`
        (bind _asbp_obstacles_wall (cast `/Game/Runner/Obtacle/BP_Obstacles_Wall` OtherActor))
        (`self.K2_DestroyActor` _asbp_obstacles_wall))
      (:`then_1`
        (bind _asbp_obstacles_blocker (cast `/Game/Runner/Obtacle/BP_Obstacles_Blocker` OtherActor))
        (`self.K2_DestroyActor` _asbp_obstacles_blocker))
      (:`then_2`
        (bind _asbp_obstacles_car_1 (cast `/Game/Runner/Obtacle/BP_Obstacles_Car1` OtherActor))
        (`self.K2_DestroyActor` _asbp_obstacles_car_1))
      (:`then_3`
        (bind _asbp_obstacles_car_2 (cast `/Game/Runner/Obtacle/BP_Obstacles_Car2` OtherActor))
        (`self.K2_DestroyActor` _asbp_obstacles_car_2))
      (:`then_4`
        (bind _asbp_obstacles_car_3 (cast `/Game/Runner/Obtacle/BP_Obstacles_Car3` OtherActor))
        (`self.K2_DestroyActor` _asbp_obstacles_car_3))
      (:`then_5`
        (bind _asbp_obstacles_car_4 (cast `/Game/Runner/Obtacle/BP_Obstacles_Car4` OtherActor))
        (`self.K2_DestroyActor` _asbp_obstacles_car_4)))
    (`KismetSystemLibrary.Delay` 1.0)
    (`self.K2_DestroyActor`)
    (else
      (`self.K2_DestroyActor`))))

(fn `UserConstructionScript`)